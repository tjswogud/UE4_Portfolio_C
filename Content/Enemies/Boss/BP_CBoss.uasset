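; BP_CBoss is a boss enemy Blueprint that seeds its AI state and shows that state as text.
; BeginPlay sets AIBossState to Approach and writes it to the BossState key of the AI controller's Blackboard.
; Every Tick reads that key back and displays the enum name on AIBossStateType, apparently as a debug readout.
; A weapon-type print and a Behavior key read are left unused.
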(event `self.ReceiveBeginPlay`
  (bind _output_get (set `self.AIBossState` "Approach"))
  (`BlackboardComponent.SetValueAsEnum` (`AIBlueprintHelperLibrary.GetBlackboard` (`AIBlueprintHelperLibrary.GetAIController` self)) "BossState" _output_get))

(event `self.ReceiveTick`
  (params (DeltaSeconds :type "Float (single-precision)"))
  (`TextRenderComponent.K2_SetText` (`self.AIBossStateType`) (`KismetTextLibrary.Conv_StringToText` (`|GetEnumeratorNameAsString` (cast `EAIStateBossType` (`BlackboardComponent.GetValueAsEnum` (`AIBlueprintHelperLibrary.GetBlackboard` (`AIBlueprintHelperLibrary.GetAIController` self)) "BossState"))))))

(fn `UserConstructionScript`)