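; BP_CEnemy_AllyMelee is a melee ally AI character that arms a sword when play begins.
; It plays a katana idle transition montage, then writes a WaitPoint state to its Blackboard and raises walk speed.
; It moves to a randomly chosen actor from its Wait array and, on arrival, switches the Blackboard AIState to Patrol.
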(event `self.ReceiveBeginPlay`
  (`|ExecutionSequence`
    (:`then_0`
      (set `CWeaponComponent.Type` "Sword" (`self.Weapons`))
      (`self.PlayAnimMontage` "/Game/Character/Montages/Ally_Melee/Katana_Blade_Idle_A_to_B_Montage.Katana_Blade_Idle_A_to_B_Montage"))
    (:`then_1`
      (bind _output_get (set `self.AIState` "WaitPoint"))
      (`BlackboardComponent.SetValueAsEnum` (`AIBlueprintHelperLibrary.GetBlackboard` (`AIBlueprintHelperLibrary.GetAIController` self)) "AIState" _output_get)
      (set `CharacterMovementComponent.MaxWalkSpeed` 1000.0 (`self.CharacterMovement`))
      (`|AIMoveTo` self (0.0 0.0 0.0) (`|ConvertAsset` (`|GetArrayItem` (`self.wait`) (`KismetMathLibrary.RandomIntegerInRange` 0 2)))
        (:`OnSuccess`
          (bind _output_get_2 (set `self.AIState` "Patrol"))
          (`BlackboardComponent.SetValueAsEnum` (`AIBlueprintHelperLibrary.GetBlackboard` (`AIBlueprintHelperLibrary.GetAIController` self)) "AIState" _output_get_2))))))

(fn `UserConstructionScript`)