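; BP_CAttachment_Sword is the sword's attachment Blueprint, switching the visual between holstered and in-hand states on the owning character.
; On BeginPlay it attaches to the sheath socket and pins a separate Foot component to the right foot's ball socket.
; Equipping moves Weapon to the hand socket, shows it and hides InvisibleSword.
; Unequipping calls AttachTo for the sheath and hides Weapon, without restoring InvisibleSword's visibility.
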(event `self.ReceiveBeginPlay`
  (`self.AttachTo` "Holster_Sheath")
  (`SceneComponent.K2_AttachToComponent` (`self.Foot`) (`Character.Mesh` (`self.OwnerCharacter`)) "ball_r" "KeepRelative" "KeepRelative" "KeepRelative" true))

(event `self.OnBeginEquip`
  (`SceneComponent.K2_AttachToComponent` (`self.Weapon`) (`Character.Mesh` (`self.OwnerCharacter`)) "Hand_Sword" "KeepRelative" "KeepRelative" "KeepRelative" true)
  (`SceneComponent.SetVisibility` (`self.InvisibleSword`) false false)
  (`SceneComponent.SetVisibility` (`self.Weapon`) true false))

(event `self.OnUnequip`
  (`self.AttachTo` "Holster_Sheath")
  (`SceneComponent.SetVisibility` (`self.Weapon`) false false))

(fn `UserConstructionScript`)