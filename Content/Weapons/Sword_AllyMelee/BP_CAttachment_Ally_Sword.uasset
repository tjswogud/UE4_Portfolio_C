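; Weapon attachment Blueprint for an ally's melee sword that moves the visible sword between holster and hand.
; On BeginPlay and on unequip, it attaches to the Holster_Sword socket and shows the Weapon component.
; When equipping begins, it attaches the Weapon component to the Hand_Sword socket on the owner character's mesh, keeping relative transforms.
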(event `self.ReceiveBeginPlay`
  (`self.AttachTo` "Holster_Sword" :!label _label)
  (`SceneComponent.SetVisibility` (`self.Weapon`) true false))

(event `self.OnBeginEquip`
  (`SceneComponent.K2_AttachToComponent` (`self.Weapon`) (`Character.Mesh` (`self.OwnerCharacter`)) "Hand_Sword" "KeepRelative" "KeepRelative" "KeepRelative" true)
  (`SceneComponent.SetVisibility` (`self.Weapon`) true false))

(event `self.OnUnequip`
  (goto _label))

(fn `UserConstructionScript`)