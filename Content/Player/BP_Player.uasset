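; Player character Blueprint that refreshes its on-character status displays every Tick.
; It writes the current state type from its state object to a text display, then casts the HealthBar widget to WB_PlayerHPbar.
; That widget receives health from the status object and resource values from CurRes and MaxRes.
; Groggy bar update and katana combo montage logic exist but are disconnected, and the construction script is empty.
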(event `Key|Eight`
  (params (Key :type "Key Structure")))

(event `self.ReceiveTick`
  (params (DeltaSeconds :type "Float (single-precision)"))
  (bind _returnvalue (`self.GetStatus`))
  (`|ExecutionSequence`
    (:`then_0`
      (`TextRenderComponent.K2_SetText` (`self.StateType`) (`KismetTextLibrary.Conv_StringToText` (`CStateComponent.GetCurType` (`self.GetState`)))))
    (:`then_1`
      (bind _aswb_player_hpbar (cast `/Game/Widgets/WB_PlayerHPbar` (`WidgetComponent.GetWidget` (`self.HealthBar`))))
      (`/Game/Widgets/WB_PlayerHPbar.Update_HealthBar` _aswb_player_hpbar (`CStatusComponent.GetHealth` _returnvalue) (`CStatusComponent.GetMaxHealth` _returnvalue))
      (`/Game/Widgets/WB_PlayerHPbar.UpdateResourceBar` _aswb_player_hpbar (`self.CurRes`) (`self.MaxRes`)))))

(fn `UserConstructionScript`)